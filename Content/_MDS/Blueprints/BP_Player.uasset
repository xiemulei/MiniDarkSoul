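; BP_Player is the player character Blueprint, handling Enhanced Input for movement, camera control and sprinting.
; Movement follows control-rotation yaw, and camera input drives controller yaw and inverted pitch.
; Holding the dodge/jump/sprint action past a threshold calls StartSprinting, which raises walk speed and messages the mesh's AnimInstance to increase play rate.
; Dodge, jump and sprint stopping are not implemented here.
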(event `self.ReceiveBeginPlay`)

(event `EnhancedInput|/Game/_MDS/Misc/Input/IA_Movement`
  (params (ActionValue :type "Vector2D Structure") (ElapsedSeconds :type "Float (double-precision)") (TriggeredSeconds :type "Float (double-precision)") (InputAction :type "InputAction Object Reference" :default "/Game/_MDS/Misc/Input/IA_Movement.IA_Movement"))
  (bind (_returnvalue_roll _returnvalue_pitch _returnvalue_yaw) (`KismetMathLibrary.BreakRotator` (`self.GetControlRotation`)))
  (bind (_x _y) (`KismetMathLibrary.BreakVector2D` ActionValue))
  ; 控制角色移动
  (:`Triggered`
    (`self.AddMovementInput` (`KismetMathLibrary.GetForwardVector` (`KismetMathLibrary.MakeRotator` 0.0 0.0 _returnvalue_yaw)) _x)
    (`self.AddMovementInput` (`KismetMathLibrary.GetRightVector` (`KismetMathLibrary.MakeRotator` 0.0 0.0 _returnvalue_yaw)) _y)))

(event `EnhancedInput|/Game/_MDS/Misc/Input/IA_CameraControl`
  (params (ActionValue :type "Vector2D Structure") (ElapsedSeconds :type "Float (double-precision)") (TriggeredSeconds :type "Float (double-precision)") (InputAction :type "InputAction Object Reference" :default "/Game/_MDS/Misc/Input/IA_CameraControl.IA_CameraControl"))
  (bind (_x _y) (`KismetMathLibrary.BreakVector2D` ActionValue))
  ; 控制摄像机
  (:`Triggered`
    (`self.AddControllerYawInput` _x) ; 水平方向
    (`self.AddControllerPitchInput` (* _y -1.0)) ; 垂直方向
  ))

(event `EnhancedInput|/Game/_MDS/Misc/Input/IA_DodgeJumpSprint`
  (params (ActionValue :type Boolean) (ElapsedSeconds :type "Float (double-precision)") (TriggeredSeconds :type "Float (double-precision)") (InputAction :type "InputAction Object Reference" :default "/Game/_MDS/Misc/Input/IA_DodgeJumpSprint.IA_DodgeJumpSprint"))
  (:`Triggered`
    (if (> ElapsedSeconds 0.8)
      (`self.StartSprinting`))))

(fn `GetAninInstance`
  (returns (ReturnValue :type "AnimInstance Object Reference"))
  (return (`SkeletalMeshComponent.GetAnimInstance` (`self.Mesh`))))

(fn `StartSprinting`
  (set `CharacterMovementComponent.MaxWalkSpeed` 600.0 (`self.CharacterMovement`))
  (message `/Game/_MDS/Blueprints/BPI/BPI_Anim.INT_SetPlayRate` (`self.GetAninInstance`) 2.0))

(fn `UserConstructionScript`)